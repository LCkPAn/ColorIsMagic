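; BP_RenderTarget_PaintingCanvas is a paintable mesh canvas that draws brush strokes into a runtime render target.
; BeginPlay clears the template target, creates a matching one, and feeds it to dynamic brush and base materials, applying the latter to the mesh.
; Paint converts a hit to UV, passes it with a validity flag to the brush, and draws that material onto the target.
; Tick repeats this draw; the camera-trace debug code is unconnected.
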(event `self.ReceiveBeginPlay`
  (bind _paintingrendertarget (`self.PaintingRenderTarget`))
  (bind _paintingrendertarget_2 (`self.PaintingRenderTarget`))
  (`|ExecutionSequence`
    (:`then_0`
      (`KismetRenderingLibrary.ClearRenderTarget2D` _paintingrendertarget_2 (`TextureRenderTarget2D.ClearColor` _paintingrendertarget_2)))
    (:`then_1`
      (bind _returnvalue (`KismetRenderingLibrary.CreateRenderTarget2D` (`TextureRenderTarget2D.SizeX` _paintingrendertarget) (`TextureRenderTarget2D.SizeY` _paintingrendertarget) (`TextureRenderTarget2D.RenderTargetFormat` _paintingrendertarget) (`TextureRenderTarget2D.ClearColor` _paintingrendertarget) (`TextureRenderTarget2D.bAutoGenerateMips` _paintingrendertarget)))
      (set `self.PaintingRenderTarget_Copy` _returnvalue))
    (:`then_2`
      (bind _returnvalue_2 (`KismetMaterialLibrary.CreateDynamicMaterialInstance` (`self.BrushMaterialTemplate`) "BrushMathInstance"))
      (bind _output_get (set `self.BrushMaterialInstance` _returnvalue_2))
      (`MaterialInstanceDynamic.SetTextureParameterValue` _output_get "RenderTarget" (`self.PaintingRenderTarget_Copy`)))
    (:`then_3`
      (bind _returnvalue_3 (`KismetMaterialLibrary.CreateDynamicMaterialInstance` (`self.BaseMaterial`) "BaseMaterialInstance"))
      (bind _output_get_2 (set `self.BaseMaterialInstance` _returnvalue_3))
      (`MaterialInstanceDynamic.SetTextureParameterValue` _output_get_2 "RenderTarget" (`self.PaintingRenderTarget_Copy`))
      (`PrimitiveComponent.SetMaterial` (`self.StaticMesh`) 0 (`self.BaseMaterialInstance`)))))

(event `/Game/FirstPerson/Blueprints/BPI_Paint.Paint`
  (params (Hit :type "HitResult Structure"))
  (bind (_uv _returnvalue) (`GameplayStatics.FindCollisionUV` Hit))
  (`MaterialInstanceDynamic.SetVectorParameterValue` (`self.BrushMaterialInstance`) "BrushPositionUV" (make `LinearColor` (`KismetMathLibrary.BreakVector2D` _uv) (`.Y` (`KismetMathLibrary.BreakVector2D` _uv)) (`KismetMathLibrary.Conv_BoolToDouble` _returnvalue) 1.0) :!label _label)
  (bind (_canvas _size _context) (`KismetRenderingLibrary.BeginDrawCanvasToRenderTarget` (`self.PaintingRenderTarget_Copy`)))
  (`Canvas.K2_DrawMaterial` _canvas (`self.BrushMaterialInstance`) (0.0 0.0) _size (0.0 0.0) (1.0 1.0) 0.0 (0.5 0.5))
  (`KismetRenderingLibrary.EndDrawCanvasToRenderTarget` _context))

(event `self.ReceiveTick`
  (params (DeltaSeconds :type "Float (single-precision)"))
  (goto _label))

(fn `UserConstructionScript`)